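; Enemy melee attack ability that plays a random tagged montage from the avatar and damages nearby live players.
; The montage's gameplay event triggers a small radial query at its combat socket, applying damage to non-friendly targets.
; Each hit fires a MeleeImpact gameplay cue carrying the montage tag, so the cue can pick its sound.
; The ability ends when the montage completes, blends out or is interrupted or cancelled.
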(event Ability|EventActivateAbility
  (bind _returnvalue (Ability|GetAvatarActorfromActorInfo))
  (bind _returnvalue_2 (Class|CombatInterface|GetAttackMontages(Message) (Ability|GetAvatarActorfromActorInfo)))
  (Variables|Default|SetTaggedMontage (Class|AuraDamageGameplayAbility|GetRandomTaggedMontagefromArray _returnvalue_2))
  (|PlayMontageandWaitProxy "None" (.montage (Variables|Default|GetTaggedMontage)) 1.0 "None" true 1.0 0.0 false
    (:then
      (Ability|Tasks|WaitGameplayEvent (.montagetag (Variables|Default|GetTaggedMontage)) 0 true
        (:EventReceived
          (bind _returnvalue_3 (Class|CombatInterface|GetCombatSocketLocation(Message) _returnvalue (.sockettag (Variables|Default|GetTaggedMontage))))
          (Variables|Default|SetCombatLocation _returnvalue_3)
          (bind _outactors (Class|AuraAbilitySystemFunctionLibrary|GetLivePlayerswithinRadius _returnvalue 45.0 (Utilities|Array|MakeArray _returnvalue) (Variables|Default|GetCombatLocation)))
          (for _array_element _outactors
            (Variables|Default|SetTargetActor _array_element)
            (if (Class|AuraAbilitySystemFunctionLibrary|IsNotFriend (Ability|GetAvatarActorfromActorInfo) (Variables|Default|GetTargetActor))
              (Class|AuraDamageGameplayAbility|CauseDamage (Variables|Default|GetTargetActor))
              (Class|GameplayAbility|ExecuteGameplayCuewithParams "(TagName=\"GameplayCue.MeleeImpact\")" (Ability|GameplayCue|MakeGameplayCueParameters :AggregatedSourceTags (GameplayTags|MakeGameplayTagContainerfromTag (.montagetag (Variables|Default|GetTaggedMontage))) :Location (Variables|Default|GetCombatLocation) :Instigator (Ability|GetAvatarActorfromActorInfo) :SourceObject (Variables|Default|GetTargetActor))))))))
    (:OnCompleted
      (Ability|EndAbility :!label _label))
    (:OnBlendOut
      (goto _label))
    (:OnInterrupted
      (goto _label))
    (:OnCancelled
      (goto _label))))

(event Ability|EventOnEndAbility
  (params (bWasCancelled :type Boolean)))