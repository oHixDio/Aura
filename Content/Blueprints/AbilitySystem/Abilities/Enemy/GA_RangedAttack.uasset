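; Enemy ranged attack Gameplay Ability that fires a projectile at the avatar's current combat target.
; It plays a random tagged montage from the avatar's attack montages and waits once for that montage's gameplay event tag.
; On that event, it spawns the projectile from the montage's socket tag toward the target's location, or ends if the target is invalid.
; The ability also ends when the montage completes, blends out, or is interrupted or cancelled.
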(event Ability|EventActivateAbility
  (bind _returnvalue (Class|CombatInterface|GetAttackMontages(Message) (Ability|GetAvatarActorfromActorInfo)))
  (Variables|Default|SetTaggedMontage (Class|AuraDamageGameplayAbility|GetRandomTaggedMontagefromArray _returnvalue))
  (|PlayMontageandWaitProxy "None" (.montage (Variables|Default|GetTaggedMontage)) 1.0 "None" true 1.0 0.0 false
    (:then
      (Ability|Tasks|WaitGameplayEvent (.montagetag (Variables|Default|GetTaggedMontage)) 0 true
        (:EventReceived
          (bind _returnvalue_2 (Class|EnemyInterface|GetCombatTarget(Message) (Ability|GetAvatarActorfromActorInfo)))
          (Utilities|IsValid _returnvalue_2
            (:Is%20Valid
              (Class|AuraProjectileSpell|SpawnProjectile (Transformation|GetActorLocation _returnvalue_2) (.sockettag (Variables|Default|GetTaggedMontage))))
            (:Is%20Not%20Valid
              (Ability|EndAbility))))))
    (:OnCompleted
      (Ability|EndAbility :!label _label))
    (:OnBlendOut
      (goto _label))
    (:OnInterrupted
      (goto _label))
    (:OnCancelled
      (goto _label))))

(event Ability|EventOnEndAbility
  (params (bWasCancelled :type Boolean)))