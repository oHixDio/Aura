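; Enemy gameplay ability that plays the shaman summon montage and spawns random minions at shuffled spawn locations.
; The first montage event shows a ground summon effect at every location.
; The second spawns AI-controlled minions one by one through a short-delay loop, each facing away from the summoner.
; Interface messages initialise each minion and raise the summoner's minion count, which drops when a minion is destroyed.
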(event Custom|OnDestroyed_イベント
  (params (DestroyedActor :type Actor%20Object%20Reference))
  (Class|EnemyInterface|DecrementMinionCount(Message) (Ability|GetAvatarActorfromActorInfo)))

(event Ability|EventActivateAbility
  (Variables|Default|SetSpawnIndex 0)
  (Utilities|Array|Clear (Variables|Default|GetSpawnLocations))
  (bind _returnvalue (Class|SummonAbility|GetSpawnLocations))
  (bind _output_get (Variables|Default|SetSpawnLocations _returnvalue))
  (Utilities|Array|Shuffle _output_get)
  (|PlayMontageandWaitProxy "None" "/Game/Assets/Enemies/Shaman/Animations/AM_Shaman_Summon.AM_Shaman_Summon" 1.0 "None" true 1.0 0.0 false
    (:then
      (Ability|Tasks|WaitGameplayEvent "(TagName=\"Events.Montage.1\")" 0 true
        (:then
          (Ability|Tasks|WaitGameplayEvent "(TagName=\"Events.Montage.2\")" 0 true
            (:EventReceived
              (if (< (Variables|Default|GetSpawnIndex) (Utilities|Array|Length (Variables|Default|GetSpawnLocations))) :!label _label
                (bind _returnvalue_2 (Game|SpawnActorfromClass (Class|SummonAbility|GetRandomSpawnMinion) (Math|Transform|MakeTransform (+ (Utilities|Array|Get(acopy) (Variables|Default|GetSpawnLocations) (Variables|Default|GetSpawnIndex)) "0.000000,0.000000,70.000000") (Math|Rotator|FindLookatRotation (Transformation|GetActorLocation (Ability|GetAvatarActorfromActorInfo)) (+ (Utilities|Array|Get(acopy) (Variables|Default|GetSpawnLocations) (Variables|Default|GetSpawnIndex)) "0.000000,0.000000,70.000000")) "1.000000,1.000000,1.000000") "AlwaysSpawn" "MultiplyWithRoot" 0 0))
                (Game|AssignOnDestroyed _returnvalue_2 (delegate Custom|OnDestroyed_イベント))
                (Pawn|SpawnDefaultController _returnvalue_2)
                (Class|EnemyInterface|Spawning(Message) _returnvalue_2)
                (Class|EnemyInterface|IncrementMinionCount(Message) (Ability|GetAvatarActorfromActorInfo))
                (Math|Integer|IncrementInt (Variables|Default|GetSpawnIndex)
                  (:%20%20
                    (Class|EnemyInterface|GetMinionCount(Message) (Ability|GetAvatarActorfromActorInfo))
                    (Utilities|FlowControl|Delay 0.2)
                    (goto _label)))))))
        (:EventReceived
          (for _array_element (Variables|Default|GetSpawnLocations)
            (Niagara|SpawnSystematLocation "/Game/Assets/Effects/Combat/NS_GroundSummon.NS_GroundSummon" _array_element)))))))

(event Ability|EventOnEndAbility
  (params (bWasCancelled :type Boolean)))