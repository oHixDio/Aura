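; GA_HitReact is a gameplay ability that makes its owning avatar react to being hit.
; On activation it applies GE_HitReact and stores the handle, then gets a montage from the avatar through a message call and plays it.
; The ability ends when the montage completes, is interrupted or cancelled, or immediately if none is valid.
; On end it removes the stored effect, so it lasts only for the reaction.
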(event Ability|EventActivateAbility
  (bind _returnvalue (Ability|ApplyGameplayEffectToOwner "/Game/Blueprints/AbilitySystem/Effects/Damage/GE_HitReact.GE_HitReact_C"))
  (Variables|Default|SetActiveHitReact _returnvalue)
  (bind _returnvalue_2 (Class|CombatInterface|GetHitReactMontage(Message) (Ability|GetAvatarActorfromActorInfo)))
  (Utilities|IsValid _returnvalue_2
    (:Is%20Valid
      (|PlayMontageandWaitProxy "None" _returnvalue_2 1.0 "None" true 1.0 0.0 false
        (:OnCompleted
          _)
        (:OnInterrupted
          _)
        (:OnCancelled
          _))
      (Ability|EndAbility))
    (:Is%20Not%20Valid
      (Ability|EndAbility))))

(event Ability|EventOnEndAbility
  (params (bWasCancelled :type Boolean))
  (Ability|RemoveGameplayEffectFromOwnerWithHandle (Variables|Default|GetActiveHitReact)))