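; GA_MeleeAttack is a gameplay ability that performs a melee attack by the avatar actor.
; It plays a random tagged montage from the avatar and waits for that montage's gameplay event.
; On the event, it damages non-friendly live players in a small radius around the tag's combat socket, debug-printing that location.
; The ability ends when the montage finishes, blends out or is interrupted or cancelled, or if none exist.
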(event Ability|EventActivateAbility
  (bind _returnvalue (Ability|GetAvatarActorfromActorInfo))
  (bind _returnvalue_2 (Class|CombatInterface|GetAttackMontages(Message) (Ability|GetAvatarActorfromActorInfo)))
  (if (> (Utilities|Array|Length _returnvalue_2) 0)
    (bind _output_get (Variables|Default|SetTaggedMontage (Utilities|Array|Get(acopy) _returnvalue_2 (Math|Random|RandomIntegerinRange 0 (- (Utilities|Array|Length _returnvalue_2) 1)))))
    (|PlayMontageandWaitProxy "None" (.Montage (Utilities|Struct|BreakTaggedMontage _output_get)) 1.0 "None" true 1.0 0.0 false
      (:then
        (Ability|Tasks|WaitGameplayEvent (.montagetag (Variables|Default|GetTaggedMontage)) 0
          (:EventReceived
            (bind _returnvalue_3 (Class|CombatInterface|GetCombatSocketLocation(Message) _returnvalue (.montagetag (Variables|Default|GetTaggedMontage))))
            (Development|PrintString (Utilities|String|ToString(Vector) _returnvalue_3))
            (bind _outactors (Class|AuraAbilitySystemFunctionLibrary|GetLivePlayerswithinRadius _returnvalue 45.0 (Utilities|Array|MakeArray _returnvalue) _returnvalue_3))
            (for _array_element _outactors
              (bind _returnvalue_4 (Class|AuraAbilitySystemFunctionLibrary|IsNotFriend (Ability|GetAvatarActorfromActorInfo) _array_element))
              (if _returnvalue_4
                (Class|AuraDamageGameplayAbility|CauseDamage _array_element))))))
      (:OnCompleted
        (Ability|EndAbility :!label _label))
      (:OnBlendOut
        (goto _label))
      (:OnInterrupted
        (goto _label))
      (:OnCancelled
        (goto _label)))
    (else
      (Ability|EndAbility))))

(event Ability|EventOnEndAbility
  (params (bWasCancelled :type Boolean)))