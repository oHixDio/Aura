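; BP_FlamePillar is a dungeon flame pillar actor whose point light flickers continuously.
; On BeginPlay it randomly picks one of two intensity timelines, and each one picks again when it finishes, forming an endless loop.
; Timeline updates feed ScaleFlameInsensity, which sets the point light's intensity to the curve value multiplied by BaseIntensity.
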(event Custom|ChoseFlame
  (switch int (Math|Random|RandomInteger 2)
    (:Default
      (CallFunction|StartFlame2 :!label _label))
    (:0
      (CallFunction|StartFlame1))
    (:1
      (goto _label))))

(event Custom|StartFlame%202
  (bind _intensity (Timeline|Intensity%202 Play)
    (:Update
      (CallFunction|ScaleFlameInsensity _intensity))
    (:Finished
      (CallFunction|ChoseFlame))))

(event Custom|StartFlame%201
  (bind _intensity (Timeline|Intensity Play)
    (:Update
      (CallFunction|ScaleFlameInsensity _intensity))
    (:Finished
      (CallFunction|ChoseFlame))))

(event EventBeginPlay
  (CallFunction|ChoseFlame))

(fn ConstructionScript)

(fn ScaleFlameInsensity
  (params (Insensity :type Float%20%28double-precision%29))
  (Rendering|Components|Light|SetIntensity (Variables|Default|GetPointLight) (* Insensity (Variables|Default|GetBaseIntensity))))