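; Dungeon actor whose mesh fades out and back in by playing or reversing a timeline that drives a "Fade" material parameter.
; The construction script caches original materials and builds dynamic instances from FadeMaterials, which FadeOut swaps onto the mesh.
; When the timeline finishes at full Fade, the original materials return.
; With BlockVisibility set, the mesh blocks the Visibility channel at full Fade and ignores it once faded out.
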(event EventBeginPlay
  (if (Variables|Default|GetBlockVisibility)
    (Collision|SetCollisionResponsetoChannel (Variables|Default|GetMesh) "ECC_Visibility" "ECR_Block")
    (else
      (Collision|SetCollisionResponsetoChannel (Variables|Default|GetMesh) "ECC_Visibility" "ECR_Ignore"))))

(event EventFadeOut
  (CallFunction|SetDynamicMateriaInstances)
  (bind _fade (Timeline|FadeScale Play)
    (:Update
      (for _array_element (Variables|Default|GetDynamicMaterialInstances)
        (Rendering|Material|SetScalarParameterValue _array_element "Fade" _fade :!class /Script/Engine.MaterialInstanceDynamic)))
    (:Finished
      (CallFunction|FadeFinished _fade))))

(event EventFadein
  (bind _fade (Timeline|FadeScale Reverse)
    (:Update
      (for _array_element (Variables|Default|GetDynamicMaterialInstances)
        (Rendering|Material|SetScalarParameterValue _array_element "Fade" _fade :!class /Script/Engine.MaterialInstanceDynamic)))
    (:Finished
      (CallFunction|FadeFinished _fade))))

(fn ConstructionScript
  (Utilities|Array|Clear (Variables|Default|GetDynamicMaterialInstances))
  (Variables|Default|SetOriginalMaterials (Rendering|Material|GetMaterials (Variables|Default|GetMesh)))
  (for _array_element (Variables|Default|GetFadeMaterials)
    (bind _returnvalue (Rendering|Material|CreateDynamicMaterialInstance _array_element "None" "None" :!class /Script/Engine.KismetMaterialLibrary))
    (Utilities|Array|AddUnique (Variables|Default|GetDynamicMaterialInstances) _returnvalue)))

(fn SetDynamicMateriaInstances
  (for (_array_element _array_index) (Variables|Default|GetDynamicMaterialInstances)
    (Rendering|Material|SetMaterial (Variables|Default|GetMesh) _array_index _array_element)))

(fn ResetMaterials
  (for (_array_element _array_index) (Variables|Default|GetOriginalMaterials)
    (Rendering|Material|SetMaterial (Variables|Default|GetMesh) _array_index _array_element)))

(fn FadeFinished
  (params (Fade :type Float%20%28double-precision%29))
  (bind _blockvisibility (Variables|Default|GetBlockVisibility))
  (if (>= Fade 1.0)
    (CallFunction|ResetMaterials)
    (if _blockvisibility
      (Collision|SetCollisionResponsetoChannel (Variables|Default|GetMesh) "ECC_Visibility" "ECR_Block"))
    (elif (>= Fade 0.0)
      (if _blockvisibility
        (Collision|SetCollisionResponsetoChannel (Variables|Default|GetMesh) "ECC_Visibility" "ECR_Ignore")))))