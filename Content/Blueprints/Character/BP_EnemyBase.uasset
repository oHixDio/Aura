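; Base enemy character Blueprint that supplies visual effects for spawning and dissolving, plus target facing.
; Separate weapon and mesh Timelines drive the Dissolve parameter on dynamic material instances passed into their events.
; SetFacingTarget feeds a location to Motion Warping as the FacingTarget warp target.
; Spawning plays a Timeline that tweens the actor's uniform scale, while BeginPlay, Tick and the construction script stay empty.
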(event EventBeginPlay)

(event Collision|EventActorBeginOverlap
  (params (OtherActor :type Actor%20Object%20Reference)))

(event EventTick
  (params (DeltaSeconds :type Float%20%28single-precision%29)))

(event EventStartWeaponDissolveTimeLine
  (params (DynamicMaterialInstance :type Material%20Instance%20Dynamic%20Object%20Reference))
  (bind _dissolve (Timeline|WeaponDissolveTimeLine Play)
    (:Update
      (Rendering|Material|SetScalarParameterValue DynamicMaterialInstance "Dissolve" _dissolve :!class /Script/Engine.MaterialInstanceDynamic))))

(event EventStartMeshDissolveTimeLine
  (params (DynamicMaterialInstance :type Material%20Instance%20Dynamic%20Object%20Reference))
  (bind _dissolve (Timeline|MeshDissolveTimeLine Play)
    (:Update
      (Rendering|Material|SetScalarParameterValue DynamicMaterialInstance "Dissolve" _dissolve :!class /Script/Engine.MaterialInstanceDynamic))))

(event EventSetFacingTarget
  (params (TargetLocation :type Vector%20%28by%20ref%29 :default "0, 0, 0"))
  (Class|MotionWarpingComponent|AddorUpdateWarpTargetfromLocation (Variables|Default|GetMotionWarping) "FacingTarget" TargetLocation))

(event EventSpawning
  (bind _scalevalue (Timeline|SpawnTweening Play)
    (:Update
      (Transformation|SetActorScale3D (Math|Conversions|ToVector(Float) _scalevalue)))))

(fn ConstructionScript)